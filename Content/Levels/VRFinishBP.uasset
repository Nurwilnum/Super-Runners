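; VR finish Blueprint with three overlap boxes for restarting the level, advancing to the next and ending a race.
; The restart box calls the GameInstance to restart on any overlap, as both branches of its player check continue.
; The next-level box calls NextLevel only for player 0's character.
; The end-race box flags a Triggered FirstPersonCharacter as EndedRace, clearing its Triggered and Fallen flags.
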(event `self.Box_Resstart.OnComponentBeginOverlap`
  (params (OverlappedComponent :type "PrimitiveComponent Object Reference") (OtherActor :type "Actor Object Reference") (OtherComp :type "PrimitiveComponent Object Reference") (OtherBodyIndex :type Integer) (bFromSweep :type Boolean) (SweepResult :type "HitResult Structure (by ref)"))
  ;[1 1 1] Restart Level
  (if (== OtherActor (`GameplayStatics.GetPlayerCharacter` 0))
    _
    (else
      _))
  (bind _asgame_instance (cast `/Game/Levels/GameInstance` (`GameplayStatics.GetGameInstance`)))
  (`/Game/Levels/GameInstance.RestartCurrentlevel` _asgame_instance))

(event `self.Box_NextLevel.OnComponentBeginOverlap`
  (params (OverlappedComponent :type "PrimitiveComponent Object Reference") (OtherActor :type "Actor Object Reference") (OtherComp :type "PrimitiveComponent Object Reference") (OtherBodyIndex :type Integer) (bFromSweep :type Boolean) (SweepResult :type "HitResult Structure (by ref)"))
  ;[1 1 1] Next Level
  (if (== OtherActor (`GameplayStatics.GetPlayerCharacter` 0))
    (bind _asgame_instance (cast `/Game/Levels/GameInstance` (`GameplayStatics.GetGameInstance`)))
    (`/Game/Levels/GameInstance.Next Level` _asgame_instance)))

(event `self.Box_EndRace.OnComponentBeginOverlap`
  (params (OverlappedComponent :type "PrimitiveComponent Object Reference") (OtherActor :type "Actor Object Reference") (OtherComp :type "PrimitiveComponent Object Reference") (OtherBodyIndex :type Integer) (bFromSweep :type Boolean) (SweepResult :type "HitResult Structure (by ref)"))
  ;[1 1 1] EndRace
  (bind _asfirst_person_character (cast `/Game/FirstPersonBP/Blueprints/FirstPersonCharacter` OtherActor))
  (if (`/Game/FirstPersonBP/Blueprints/FirstPersonCharacter.Triggered` _asfirst_person_character)
    (set `/Game/FirstPersonBP/Blueprints/FirstPersonCharacter.Triggered` false _asfirst_person_character)
    (set `/Game/FirstPersonBP/Blueprints/FirstPersonCharacter.EndedRace` true _asfirst_person_character)
    (set `/Game/FirstPersonBP/Blueprints/FirstPersonCharacter.Fallen` false _asfirst_person_character)))

(fn `UserConstructionScript`)